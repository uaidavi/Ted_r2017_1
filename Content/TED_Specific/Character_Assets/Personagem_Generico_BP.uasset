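; Generic character Blueprint that handles death and declares mostly empty functions for attacks, block, riposte and respawn.
; Tick checks for zero health through Test_Is_Dead and fires DeathEvent.
; Death_Behavior rechecks death on authority only and unpossesses the Player_Controller_BP, after which DeathEvent destroys the actor, which the author's comment says notifies the controller to allow respawn.
; DoubleJump simply calls Jump.
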(event `self.ReceiveBeginPlay`)

(event `self.ReceiveTick`
  (params (DeltaSeconds :type "Float (single-precision)"))
  ;[1 1 1] Testa constantemente se o HP do personagem chegou a 0
  (`self.Test_Is_Dead`
    (:`Is_Dead`
      (`KismetSystemLibrary.PrintString` "Morri")
      (`self.DeathEvent`))))

(event `DeathEvent`
  ;[1 1 1] Executa a morte do personagem, independente do motivo
  (bind _is_dead (`self.Death_Behavior`))
  (if _is_dead
    (`self.K2_DestroyActor`) ; A destruíção do ator ativa a notificação do controlador para permitir o respawn
    (else
      (`KismetSystemLibrary.PrintString` "Can't kill that which must still live"))))

(fn `Atk1_Call`)

(fn `Atk2_Call`)

(fn `BlockCall`)

(fn `Death_Behavior`
  (returns (Is_Dead :type Boolean))
  (`/Engine/EditorBlueprintResources/ActorMacros.Switch Has Authority`
    (:`Authority`
      (`self.Test_Is_Dead` ; Teste de redundância, garante que o personagem está morto.
        (:`Is_Dead`
          ;[1 1 1] Retira a posse do controlador sobre o personagem se ele estiver morto.
          (`KismetSystemLibrary.PrintString` "Morri")
          (bind _asplayer_controller_bp (cast `/Game/TED_Specific/Character_Assets/Player_Controller_BP` (`self.GetController`))
            (:`then`
              (`Controller.UnPossess` _asplayer_controller_bp))
            (:`CastFailed`
              (`KismetSystemLibrary.PrintString` "Death Cast fail" true true (struct :`R` 1.0 :`G` 0.742836 :`B` 0.027617 :`A` 1.0) 20.0)))
          (return true) ; Retorna com um aviso de que o personagem está morto para continuar o processo de morte
        )
        (:`Is_Alive`
          _)))
    (:`Remote`
      _))
  (return false))

(fn `DoubleJump`
  (`self.Jump`))

(fn `OnRep_Health_De-Buff`)

(fn `Respawn_Behavior`)

(fn `RiposteCall`)

(fn `StringTest`
  (for _array_element _
    (`KismetSystemLibrary.PrintString` _array_element true true (struct :`G` 0.66 :`B` 1.0 :`A` 1.0) 5.0)))

(fn `UserConstructionScript`)