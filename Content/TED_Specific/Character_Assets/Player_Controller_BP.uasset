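; Player controller that drives a Personagem_Generico_BP character: movement, spring-arm camera and respawn.
; Pan input turns the pitch-clamped spring arm; side input turns the idle character or strafes when moving, and a timeline lerps control rotation to the camera when movement starts.
; Jump calls the pawn's DoubleJump.
; On pawn destruction it requests a selected-character respawn from GeneralRules, possesses it and re-fetches references, retrying while invalid.
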(event `self.ReceiveTick`
  (params (DeltaSeconds :type "Float (single-precision)"))
  ;[1 1 1] Eventos chamados a todo
  ; momento
  (`self.Char_Rot_Call`))

(event `InputAxis|PanHor`
  (params (AxisValue :type "Float (single-precision)"))
  ;[1 1 1] Rotação da câmera no eixo "x"
  (`self.Validation_Macro`
    (:`Is Valid`
      (`self.CamRotationX` (`self.Cast_Char`) AxisValue))))

(event `InputAxis|PanVert`
  (params (AxisValue :type "Float (single-precision)"))
  ;[1 1 1] Rotação da câmera no eixo "y"
  (`self.Validation_Macro`
    (:`Is Valid`
      (`self.CamRotationY` (`self.Cast_Char`) AxisValue))))

(event `Char_Rot_Call`
  ;[1 1 1] Char_Rot_Behavior
  (`self.Validation_Macro`
    (:`Is Valid`
      (if (`self.VelocityTest`)
        (if (and (`self.VelocityTest`) (`self.StartedMov`))
          (bind _char_initial_rot (`self.Create_Char_InitialRot`)
            (:`Exec`
              (set `self.Char_Init_Rot` _char_initial_rot)
              (bind (_direction _rot_alpha) (`Timeline|Timeline_0` :!via `PlayFromStart`)
                (:`Update`
                  (`self.SetControlRotation` (`KismetMathLibrary.RLerp` (`self.Char_Init_Rot`) (`SceneComponent.RelativeRotation` (`self.CamHold`)) _rot_alpha true))
                  (set `self.StartedMov` false))))))
        (else
          ;;[1 1 1] RestartStartedMoving
          (set `self.StartedMov` true))))))

(event `InputAxis|RunForward`
  (params (AxisValue :type "Float (single-precision)"))
  ;[1 1 1] Movimentação do personagem para frente e para trás
  (`self.Validation_Macro`
    (:`Is Valid`
      (`self.MoveForward` (`self.Cast_Char`) AxisValue))))

(event `InputAxis|MoveTurnSide`
  (params (AxisValue :type "Float (single-precision)"))
  ;[1 1 1] Movimentação de lado ou rotação do personagem
  (`self.Validation_Macro`
    (:`Is Valid`
      (`self.MoveSideways` (`self.Cast_Char`) AxisValue))))

(event `InputAction|Jump_Inp`
  (params (Key :type "Key Structure" :default "AnyKey"))
  ;[1 1 1] Chama a função de pulo duplo do personagem (não é feito no controlador em si porque pode variar a funcionalidade)
  (:`Pressed`
    (`self.Validation_Macro`
      (:`Is Valid`
        (bind _aspersonagem_generico_bp (cast `/Game/TED_Specific/Character_Assets/Personagem_Generico_BP` (`self.K2_GetPawn`)))
        (`/Game/TED_Specific/Character_Assets/Personagem_Generico_BP.DoubleJump` _aspersonagem_generico_bp)))))

(event `RespawnReset`
  ;[1 1 1] Respawn
  ;;[1 1 1] Seta (no começo da partida) ou reseta (quando algum personagem morre) a possibilidade de um respawn
  (`KismetSystemLibrary.Delay` 0.2 :!label _label)
  (`self.GetReferences`) ; Necessário para saber qual peão está sendo utilizado
  (`self.Re/SpawnCall`)
  (`self.ProblematicReference`))

(event `self.ReceiveBeginPlay`
  ;[1 1 1] Respawn
  ;;[1 1 1] Seta (no começo da partida) ou reseta (quando algum personagem morre) a possibilidade de um respawn
  (goto _label))

(event `ProblematicReference`
  ;[1 1 1] Respawn
  ;;[1 1 1] Seta (no começo da partida) ou reseta (quando algum personagem morre) a possibilidade de um respawn
  (if (`self.InvalidRefs`)
    (goto _label)
    (else
      (`KismetSystemLibrary.PrintString` "Retirei o bug, referências OK!" true true (struct :`G` 0.66 :`B` 1.0 :`A` 1.0) 10.0))))

(event `Re/SpawnCall`
  (bind _returnvalue (`self.K2_GetPawn`))
  ;[1 1 1] Respawn
  ;;[1 1 1] Ativa o respawn ao detectar que o personagem morreu (no bind event), apenas se o personagem for válido
  (`/Engine/EditorBlueprintResources/StandardMacros.IsValid` _returnvalue
    (:`Is Valid`
      (add `self.OnDestroyed` _returnvalue (delegate `RequestServerSpawn`)))))

(event `RequestServerSpawn` :!signature `self.OnDestroyed`
  (params (DestroyedActor :type "Actor Object Reference"))
  ;[1 1 1] Respawn
  ;;[1 1 1] Ativa o respawn ao detectar que o personagem morreu (no bind event), apenas se o personagem for válido
  (`KismetSystemLibrary.Delay` 2.0)
  (`self.RespawnSequence`)
  (`self.RespawnReset`))

(event `InputAction|BotaoTeste`
  (params (Key :type "Key Structure" :default "AnyKey"))
  ;[1 1 1] Debug
  (:`Pressed`
    (bind _aspersonagem_generico_bp (cast `/Game/TED_Specific/Character_Assets/Personagem_Generico_BP` (`self.K2_GetPawn`)))
    (`KismetSystemLibrary.PrintString` "vou morrer")
    (set `/Game/TED_Specific/Character_Assets/Personagem_Generico_BP.CurHealth` 0.0 _aspersonagem_generico_bp)))

(event `OnCharacterSelection`
  (params (`CharacterSelected on menu` :type "/Game/TED_Specific/Character_Assets/Personagem_Generico_BP Class Reference"))
  (set `self.ContrSelectedCharacter` `CharacterSelected on menu`))

(fn `CamRotationX`
  (params (To_Char :type "Object Object Reference") (Axis :type "Float (double-precision)"))
  ;[1 1 1] Adiciona rotação somente na câmera se o personagem estiver parado e retorna.
  (`SceneComponent.K2_AddRelativeRotation` (`self.CamHold`) (`KismetMathLibrary.MakeRotator` 0.0 0.0 Axis) false false)
  (if (`self.VelocityTest`)
    ;[1 1 1] Adiciona rotação também sobre o personagem se ele estiver em movimento.
    (`Pawn.AddControllerYawInput` To_Char (* Axis 0.4))
    (return)
    (else
      (return))))

(fn `CamRotationY`
  (params (To_Char :type "Object Object Reference") (Axis_Value :type "Float (double-precision)"))
  (bind (_newparam _toohigh _toolow) (`self.Camera_Rot_Test`))
  (bind _camhold (`self.CamHold`))
  (bind _camhold_2 (`self.CamHold`))
  (bind (_relativerotation_roll _relativerotation_pitch _relativerotation_yaw) (`KismetMathLibrary.BreakRotator` (`SceneComponent.RelativeRotation` _camhold)))
  (bind (_relativerotation_roll_2 _relativerotation_pitch_2 _relativerotation_yaw_2) (`KismetMathLibrary.BreakRotator` (`SceneComponent.RelativeRotation` _camhold_2)))
  (`self.Validation_Macro`
    (:`Is Valid`
      (if _toohigh
        ;[1 1 1] Trava a rotação da câmera se a rotação dela em "y" for maior que -50º
        (`SceneComponent.K2_SetRelativeRotation` _camhold_2 (`KismetMathLibrary.MakeRotator` _relativerotation_roll_2 -47.99 _relativerotation_yaw_2) false false)
        (elif _toolow
          ;[1 1 1] Trava a rotação da câmera se a rotação dela em "y" for menor que -50º
          (`SceneComponent.K2_SetRelativeRotation` _camhold (`KismetMathLibrary.MakeRotator` _relativerotation_roll 47.99 _relativerotation_yaw) false false)
          (else
            ;[1 1 1] Adiciona rotação em "y" se o valor for válido.
            (`SceneComponent.K2_AddRelativeRotation` (`self.CamHold`) (`KismetMathLibrary.MakeRotator` 0.0 Axis_Value) false false)))))
    (:`Char Is Not Valid`
      _)
    (:`Cam Is Not Valid`
      _))
  (return))

(fn `ControllerDeathBehavior`
  (`self.UnPossess`)
  (bind _asgeneral_rules (cast `/Game/TED_Specific/GeneralRules` (`GameplayStatics.GetGameMode`)))
  (`/Game/TED_Specific/GeneralRules.Request_Respawn` _asgeneral_rules null))

(fn `GetReferences`
  (bind _returnvalue (`self.K2_GetPawn`))
  (`/Engine/EditorBlueprintResources/StandardMacros.IsValid` _returnvalue
    (:`Is Valid`
      (bind _aspersonagem_generico_bp (cast `/Game/TED_Specific/Character_Assets/Personagem_Generico_BP` _returnvalue)
        (:`then`
          (`/Engine/EditorBlueprintResources/StandardMacros.IsValid` _aspersonagem_generico_bp
            (:`Is Valid`
              (bind _output_get (set `self.Cast_Char` _aspersonagem_generico_bp))
              (`/Engine/EditorBlueprintResources/StandardMacros.IsValid` _output_get
                (:`Is Valid`
                  (set `self.CamHold` (`/Game/TED_Specific/Character_Assets/Personagem_Generico_BP.SpringArm` _aspersonagem_generico_bp))
                  (set `self.InvalidRefs` false))
                (:`Is Not Valid`
                  (`KismetSystemLibrary.PrintString` "Set Char Invalido" true true (struct :`G` 1.0 :`B` 0.095112 :`A` 1.0) 30.0)
                  (`KismetSystemLibrary.PrintString` "AlgoEstáInvalido" true true (struct :`R` 1.0 :`G` 0.81113 :`A` 1.0) 90.0 :!label _label)
                  (set `self.InvalidRefs` true))))
            (:`Is Not Valid`
              (goto _label))))
        (:`CastFailed`
          (goto _label))))
    (:`Is Not Valid`
      (goto _label)))
  (return))

(fn `MoveForward`
  (params (To_Char :type "Object Object Reference") (`FWD/BWD` :type "Float (double-precision)"))
  (`self.Validation_Macro` ; Testa se o personagem e câmera existem e se são válidos
    (:`Is Valid`
      (if (not (`self.IsIncapacitated`))
        (`Pawn.AddMovementInput` To_Char (`KismetMathLibrary.GetForwardVector` (`KismetMathLibrary.MakeRotator` 0.0 0.0 (.yaw (`self.GetControlRotation`)))) (* `FWD/BWD` 1.0) false)))
    (:`Char Is Not Valid`
      _)
    (:`Cam Is Not Valid`
      _))
  (return))

(fn `MoveSideways`
  (params (To_Char :type "Object Object Reference") (Axis_Value :type "Float (double-precision)"))
  (if (`self.VelocityTest`)
    ;[1 1 1] Caso o personagem esteja já em movimento é adicionado
    ; movimento lateral.
    (`Pawn.AddMovementInput` To_Char (`KismetMathLibrary.GetRightVector` (`KismetMathLibrary.MakeRotator` 0.0 0.0 (.yaw (`self.GetControlRotation`)))) Axis_Value false)
    (else
      ;[1 1 1] Caso o personagem esteja parado ele apenas rotaciona no lugar
      (`Pawn.AddControllerYawInput` To_Char Axis_Value)))
  (return))

(fn `RespawnSequence`
  (bind _asgeneral_rules (cast `/Game/TED_Specific/GeneralRules` (`GameplayStatics.GetGameMode`))
    (:`then`
      (bind _new_char (`/Game/TED_Specific/GeneralRules.Request_Respawn` _asgeneral_rules (`self.ContrSelectedCharacter`)))
      (`self.Possess` _new_char))
    (:`CastFailed`
      _))
  (return))

(fn `UserConstructionScript`)